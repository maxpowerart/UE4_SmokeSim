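; BP_NPC is an NPC that the player targets by cursor hover and can hold a dialogue with.
; Hovering swaps its sprite and sets TargetNPC on BP_PChar; leaving restores the sprite and clears the target.
; Talk switches the AI controller to BT_DialogTree; EndTalk destroys the brain component, runs BT_NPC_behaviour and clears the target.
; Tick sets the BT variable to None every frame.
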(event OnBeginCursorOver(Sprite)
  (params (TouchedComponent :type Primitive%20Component%20Object%20Reference))
  (Rendering|Components|Sprite|SetSprite (Variables|Default|GetSprite) "/Game/RandomAssets/ii2_Sprite.ii2_Sprite")
  (bind _asbp_pchar (Utilities|Casting|CastToBP_PChar (Game|Player|GetPlayerPawn 0)))
  (Variables|/Game/Characters/Main/BP_PChar.BP_PChar_C|SetTargetNPC _asbp_pchar self))

(event OnEndCursorOver(Sprite)
  (params (TouchedComponent :type Primitive%20Component%20Object%20Reference))
  (Rendering|Components|Sprite|SetSprite (Variables|Default|GetSprite) "/Game/RandomAssets/arrowWall_S_Sprite.arrowWall_S_Sprite")
  (bind _asbp_pchar (Utilities|Casting|CastToBP_PChar (Game|Player|GetPlayerPawn 0)))
  (Variables|/Game/Characters/Main/BP_PChar.BP_PChar_C|SetTargetNPC _asbp_pchar 0))

(event EventTalk
  (bind _self self)
  (bind _returnvalue (AI|GetAIController _self))
  ;[1 1 1] Начало разговора
  (AI|RunBehaviorTree _returnvalue "/Game/Mechanics/DialogueSystem/DialogTree/BT_DialogTree.BT_DialogTree")
  (Class|BrainComponent|RestartLogic (Variables|/Script/AIModule.AIController|GetBrainComponent _returnvalue)))

(event Collision|EventActorBeginOverlap
  (params (OtherActor :type Actor%20Object%20Reference)))

(event EventEndTalk
  (bind _self self)
  (bind _returnvalue (AI|GetAIController _self))
  (bind _braincomponent (Variables|/Script/AIModule.AIController|GetBrainComponent _returnvalue))
  ;[1 1 1] Конец разговора
  (Components|DestroyComponent _braincomponent)
  (AI|RunBehaviorTree (AI|GetAIController self) "/Game/Characters/NPC/BT_NPC_behaviour.BT_NPC_behaviour")
  (AI|Logic|StartLogic _braincomponent)
  (bind _asbp_pchar (Utilities|Casting|CastToBP_PChar (Game|Player|GetPlayerPawn 0)))
  (Variables|/Game/Characters/Main/BP_PChar.BP_PChar_C|SetTargetNPC _asbp_pchar 0))

(event EventTick
  (params (DeltaSeconds :type Float%20%28single-precision%29))
  (Variables|Default|SetBT 0))

(fn ConstructionScript)