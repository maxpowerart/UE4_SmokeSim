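; Main player character: a Paper2D flipbook pawn with point-and-click movement, inventory toggle and status effects added to its StatusBar.
; While Interact is held, a Tick-driven gate either moves to the cursor hit or, based on TargetItem and TargetNPC, approaches to interact or talk.
; Movement and ComeCloser flip the sprite, swap move/idle flipbooks and use MoveComponentTo with distance-based duration; ComeCloser stops short of the target.
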(event Custom|GetStatusEffect
  (params (StatusEffect :type S%20Effect%20Structure))
  (Utilities|Array|AddUnique (Variables|/Game/Mechanics/StatusSystem/BP_StatusBarComponent.BP_StatusBarComponent_C|GetEffects (Variables|Default|GetStatusBar)) StatusEffect))

(event EventBeginPlay)

(event Collision|EventActorBeginOverlap
  (params (OtherActor :type Actor%20Object%20Reference)))

(event EventTick
  (params (DeltaSeconds :type Float%20%28single-precision%29))
  (bind _backpack (Variables|Default|GetBackpack))
  (bind _inventorywindow (Variables|/Game/Mechanics/Inventory/StructsAndInterface/BP_InventoryComponent.BP_InventoryComponent_C|GetInventoryWindow _backpack))
  ;[1 1 1] Передвижение
  (Utilities|FlowControl|Gate true :!label _label
    (:Exit
      (if (== (Variables|Default|GetTargetItem) 0)
        (if (== (Variables|Default|GetTargetNPC) 0)
          (Utilities|Movement)
          (else
            ;[1 1 1] Диалог
            (bind _asbp_npc (Utilities|Casting|CastToBP_NPC (.HitActor (Collision|BreakHitResult (.HitResult (Game|Player|GetHitResultUnderCursorbyChannel (Game|GetPlayerController 0) "TraceTypeQuery1" true))))))
            (Utilities|ComeCloser)
            (Utilities|FlowControl|Sequence
              (:then_0
                (goto _label Close))
              (:then_1
                (Default|Talk _asbp_npc)))))
        (else
          ;[1 1 1] Поднятие предметов
          (bind _asbp_item (Utilities|Casting|CastToBP_Item (.HitActor (Collision|BreakHitResult (.HitResult (Game|Player|GetHitResultUnderCursorbyChannel (Game|GetPlayerController 0) "TraceTypeQuery1" true))))))
          (Utilities|ComeCloser)
          (Default|Interact _asbp_item self)
          (Variables|Default|SetTargetItem 0)
          (if (not (== _inventorywindow 0))
            (Default|Update _inventorywindow)))))))

(event Input|ActionEvents|InputActionInteract
  (params (Key :type Key%20Structure))
  (bind _backpack (Variables|Default|GetBackpack))
  (bind _inventorywindow (Variables|/Game/Mechanics/Inventory/StructsAndInterface/BP_InventoryComponent.BP_InventoryComponent_C|GetInventoryWindow _backpack))
  ;[1 1 1] Передвижение
  (:Pressed
    (Utilities|FlowControl|Gate true) ; enters at Open
  )
  (:Released
    (Utilities|FlowControl|Gate true) ; enters at Close
  ))

(event Input|ActionEvents|InputActionInventory
  (params (Key :type Key%20Structure))
  ;[1 1 1] Окно инвентаря
  (:Pressed
    (Default|ToggleInventory (Variables|Default|GetBackpack))))

(fn ConstructionScript)