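; An inventory component that keeps the owner's items in a fixed-size array of slot structs, sized on BeginPlay.
; Adding merges stackable items into the first slot of the same item class, otherwise fills an empty slot.
; Removal handles only consumables, decrementing the stack or replacing the last one with an appended empty slot.
; It also toggles a centre-anchored inventory widget on the player controller's HUD canvas; UseItem is a stub.
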(event EventBeginPlay
  (CallFunction|PrepareInventory))

(event EventTick
  (params (DeltaSeconds :type Float%20%28single-precision%29)))

(fn ToggleInventory
  (bind _inventorywindow (Variables|Default|GetInventoryWindow)
    (:then
      (Widget|RemovefromParent _inventorywindow)
      (Variables|Default|SetInventoryWindow 0))
    (:else
      (bind _returnvalue (UserInterface|CreateWidget "/Game/Mechanics/Inventory/InventoryUI/WBP_InventoryWindow.WBP_InventoryWindow_C" 0 self))
      (bind _output_get (Variables|Default|SetInventoryWindow _returnvalue))
      (bind _asbp_play_cont (Utilities|Casting|CastToBP_PlayCont (Game|GetPlayerController 0)))
      (bind _returnvalue_2 (Class|CanvasPanel|AddChildtoCanvas (Variables|/Game/Characters/Main/UI/WBP_HUD.WBP_HUD_C|GetHUDCanvas (Variables|/Game/Characters/Main/BP_PlayCont.BP_PlayCont_C|GetHUDWidget _asbp_play_cont)) _output_get))
      (Class|CanvasPanelSlot|SetAutoSize _returnvalue_2 true)
      (Class|CanvasPanelSlot|SetAlignment _returnvalue_2 "(X=0.500000,Y=0.500000)")
      (Class|CanvasPanelSlot|SetAnchors _returnvalue_2 (Utilities|Struct|MakeAnchors "(X=0.500000,Y=0.500000)" "(X=0.500000,Y=0.500000)"))
      (Class|CanvasPanelSlot|SetPosition _returnvalue_2 (Variables|Default|GetPosition)))))

(fn AddtoInventory
  (params (ContentToAdd :type S%20Slot%20Structure))
  (if (.isstackable (.itemstructure ContentToAdd))
    (bind _stackindex (Utilities|HasPartialStack ContentToAdd)
      (:True
        (bind _success (CallFunction|AddtoStack ContentToAdd _stackindex))
        (return _success))
      (:False
        _)))
  (CallFunction|CreateStack ContentToAdd)
  (return true))

(fn PrepareInventory
  (Utilities|Array|Resize (Variables|Default|GetInventory) (Variables|Default|GetNumberOfSlots)))

(fn CreateStack
  (params (ContentToAdd :type S%20Slot%20Structure))
  (bind _inventory (Variables|Default|GetInventory))
  (Utilities|Array|SetArrayElem _inventory (Utilities|Array|FindItem _inventory (Utilities|Struct|MakeSSlot "(Name_5_9389AA6944BE0488F4F59795EEEB2DC4=NSLOCTEXT(\"[750997804445684271850BB3527A2A5A]\", \"0144DB7A431EA20A391C9F99B615C8C0\", \"None\"),isStackable_6_7E5EE7D24770D63C0CA60693ADA97903=True,Thumbnail_15_10331EF14A67E063F038AAB76BDCDF88=None,Description_12_A33EE76A468FA3A4A062D09C3D13D428=NSLOCTEXT(\"[750997804445684271850BB3527A2A5A]\", \"AD9C4FE54DF8BB5890A1398300E8DEB1\", \"None\"),isConsumable_7_86D04095479A223A4D32A198EB2884CF=True,Class_16_228E45E54B9AB4E46C73098E17AAD604=None,isEquipable_18_C6AA0419449CE1B353544580BA0D0EE4=False)")) ContentToAdd))

(fn AddtoStack
  (params (SlotStructure :type S%20Slot%20Structure) (SlotIndex :type Integer))
  (bind _inventory (Variables|Default|GetInventory))
  (bind _output (Utilities|Array|Get(acopy) _inventory SlotIndex))
  (LocalVariables|SetQuantity (.quantity (Utilities|Array|Get(acopy) (Variables|Default|GetInventory) SlotIndex)))
  (Utilities|Array|SetArrayElem _inventory SlotIndex (Utilities|Struct|MakeSSlot (.itemstructure _output) (+ (.quantity _output) (.quantity SlotStructure))))
  (return true))

(fn RemovefromInventory
  (params (ContentToRemove :type S%20Slot%20Structure))
  (bind _inventory (Variables|Default|GetInventory))
  (bind _inventory_2 (Variables|Default|GetInventory))
  (bind _inventory_3 (Variables|Default|GetInventory))
  (bind _returnvalue (Utilities|Array|FindItem _inventory ContentToRemove))
  (bind _output (Utilities|Array|Get(acopy) _inventory_2 _returnvalue))
  (if (not (Utilities|Enum|Equal(Enum) (.name (.itemstructure ContentToRemove)) (Utilities|Text|MakeLiteralText "None")))
    (if (.isconsumable (.itemstructure ContentToRemove))
      (if (> (.Quantity (Utilities|Struct|BreakSSlot _output)) 1)
        (bind _success (CallFunction|DeletefromStack _output _returnvalue))
        (return _success)
        (else
          (bind _returnvalue_2 (Utilities|Array|RemoveItem _inventory_3 _output))
          (Utilities|Array|Add _inventory_3 (Utilities|Struct|MakeSSlot (Utilities|Struct|MakeSItem "None" true 0 "None")))
          (return _returnvalue_2))))))

(fn DeletefromStack
  (params (SlotStructure :type S%20Slot%20Structure) (SlotIndex :type Integer))
  (bind _inventory (Variables|Default|GetInventory))
  (bind _output (Utilities|Array|Get(acopy) _inventory SlotIndex))
  (LocalVariables|SetQuantity (.quantity (Utilities|Array|Get(acopy) (Variables|Default|GetInventory) SlotIndex)))
  (Utilities|Array|SetArrayElem _inventory SlotIndex (Utilities|Struct|MakeSSlot (.itemstructure _output) (- (.quantity _output) 1)))
  (return true))

(fn UseItem
  (params (SlotIndex :type Integer))
  (bind _inventory (Variables|Default|GetInventory))
  (bind _output (Utilities|Array|Get(acopy) _inventory SlotIndex))
  (if (or (.isconsumable (.itemstructure _output)) (.isequipable (.itemstructure _output)))
    _))