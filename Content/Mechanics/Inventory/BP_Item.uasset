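; BP_Item is a pickup item actor that can be collected into an inventory.
; Hovering the cursor over its sprite sets it as the player character's TargetItem, and leaving clears it.
; On Interact, it adds one of its ItemStructure to the interactor's BP_InventoryComponent and destroys itself if the add succeeds.
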(event OnBeginCursorOver(Sprite)
  (params (TouchedComponent :type Primitive%20Component%20Object%20Reference))
  (bind _asbp_pchar (Utilities|Casting|CastToBP_PChar (Game|Player|GetPlayerPawn 0)))
  (Variables|/Game/Characters/Main/BP_PChar.BP_PChar_C|SetTargetItem _asbp_pchar self))

(event OnEndCursorOver(Sprite)
  (params (TouchedComponent :type Primitive%20Component%20Object%20Reference))
  (bind _asbp_pchar (Utilities|Casting|CastToBP_PChar (Game|Player|GetPlayerPawn 0)))
  (Variables|/Game/Characters/Main/BP_PChar.BP_PChar_C|SetTargetItem _asbp_pchar 0))

(event EventBeginPlay)

(event Collision|EventActorBeginOverlap
  (params (OtherActor :type Actor%20Object%20Reference)))

(event EventTick
  (params (DeltaSeconds :type Float%20%28single-precision%29)))

(event EventInteract
  (params (Interactor :type Actor%20Object%20Reference))
  (bind _success (Default|AddtoInventory (Actor|GetComponentbyClass Interactor "/Game/Mechanics/Inventory/StructsAndInterface/BP_InventoryComponent.BP_InventoryComponent_C") (Utilities|Struct|MakeSSlot (Variables|Default|GetItemStructure) 1)))
  (if _success
    (Actor|DestroyActor)))

(fn ConstructionScript)